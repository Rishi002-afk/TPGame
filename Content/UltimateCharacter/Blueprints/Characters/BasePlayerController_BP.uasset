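; Base player controller that forwards pause menu input and game-over toggling to the BaseHUD_BP HUD and manages the player's score.
; AddScore multiplies points by the combo counter, clamps the total at zero and sends it to the HUD with a location-based score popup.
; Each combo increment restarts a two-second timer that resets the counter and hides its display.
; Helpers restart the level, return to the current checkpoint and fetch the player character's tag.
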(event EventBeginPlay)

(event EventTick
  (params (DeltaSeconds :type Float%20%28single-precision%29)))

(event Input|ActionEvents|InputActionPauseMenu
  (params (Key :type Key%20Structure))
  ;[1 1 1] Toggles pause menu
  (:Pressed
    (bind _asbase_hud_bp (Utilities|Casting|CastToBaseHUD_BP (HUD|GetHUD)))
    (Default|PauseMenu _asbase_hud_bp)
    (Audio|PlaySound2D "/Game/UltimateCharacter/Sounds/UI/MenuEnter03_Stereo.MenuEnter03_Stereo" 1.0 1.0 0.0 0 0)))

(event Input|ActionEvents|InputActionMenuUp
  (params (Key :type Key%20Structure))
  ;[1 1 1] Switch between main menu buttons using keyboard or gamepad
  (:Pressed
    (bind _asbase_hud_bp (Utilities|Casting|CastToBaseHUD_BP (HUD|GetHUD)))
    (Default|MoveonPauseMenu _asbase_hud_bp true)))

(event Input|ActionEvents|InputActionMenuDown
  (params (Key :type Key%20Structure))
  ;[1 1 1] Switch between main menu buttons using keyboard or gamepad
  (:Pressed
    (bind _asbase_hud_bp (Utilities|Casting|CastToBaseHUD_BP (HUD|GetHUD)))
    (Default|MoveonPauseMenu _asbase_hud_bp false)))

(event Input|ActionEvents|InputActionMenuEnter
  (params (Key :type Key%20Structure))
  ;[1 1 1] Select main menu button using Enter on keyboard or game pad bottom face button
  (:Pressed
    (bind _asbase_hud_bp (Utilities|Casting|CastToBaseHUD_BP (HUD|GetHUD)))
    (Default|SelectonPauseMenu _asbase_hud_bp)))

(fn ConstructionScript)

(fn ToggleGameOver
  (bind _asbase_hud_bp (Utilities|Casting|CastToBaseHUD_BP (HUD|GetHUD)))
  (Default|ToggleGameOver _asbase_hud_bp))

(fn ResetGameOver
  (Development|ExecuteConsoleCommand "RestartLevel" (Game|GetPlayerController 0)))

(fn AddScore
  (params (InScore :type Integer) (InLocation :type Vector))
  ;[1 1 1] Update the score and then send it to the HUD
  (Variables|Internal|SetScore (Math|Integer|Max(Integer) (+ (* InScore (Math|Integer|Max(Integer) 1 (Variables|Internal|GetComboCounter))) (Variables|Internal|GetScore))))
  (bind _asbase_hud_bp (Utilities|Casting|CastToBaseHUD_BP (HUD|GetHUD)))
  (Default|UpdateScore _asbase_hud_bp (Variables|Internal|GetScore) (Variables|Internal|GetComboCounter))
  (Default|SpawnScore _asbase_hud_bp InScore InLocation))

(fn GetPlayerTag
  (bind _asbase_character_bp (Utilities|Casting|CastToBaseCharacter_BP (Game|Player|GetPlayerPawn 0))
    (:then
      (return (Variables|/Game/UltimateCharacter/Blueprints/Characters/BaseCharacter_BP.BaseCharacter_BP_C|GetCharacterTag _asbase_character_bp)))
    (:CastFailed
      (return "Failed!"))))

(fn ResettoCheckpoint
  (Utilities|IsValid (Variables|Internal|GetCurrentCheckpoint)
    (:Is%20Valid
      (Default|ResetCheckpoint (Variables|Internal|GetCurrentCheckpoint) self))))

(fn AddScoreComboCounter
  (bind _output_get (Variables|Internal|SetComboCounter (+ (Variables|Internal|GetComboCounter) 1)))
  (Utilities|Time|ClearandInvalidateTimerbyHandle (Variables|Default|GetScoreComboTimer))
  (bind _returnvalue (Utilities|Time|SetTimerbyFunctionName self "ResetScoreComboCounter" 2.0))
  (Variables|Default|SetScoreComboTimer _returnvalue))

(fn ResetScoreComboCounter
  (Variables|Internal|SetComboCounter 1)
  (bind _asbase_hud_bp (Utilities|Casting|CastToBaseHUD_BP (HUD|GetHUD)))
  (Default|HideComboCounter _asbase_hud_bp))