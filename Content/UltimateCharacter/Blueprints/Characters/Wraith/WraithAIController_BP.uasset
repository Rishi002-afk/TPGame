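; AI controller for the Wraith character, specializing the attack range check of its parent controller.
; GetDistanceForAttack keeps the parent's result, except when one attack type is out of range with the target at or inside its minimum distance.
; In that case a landed pawn starts a jump and stays out of range, while an unlanded pawn reports the attack as in range.
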(event EventTick
  (params (DeltaSeconds :type Float%20%28single-precision%29))
  (|CallParentFunction DeltaSeconds) ; This node is disabled and will not be called.\nDrag off pins to build functionality.
)

(fn ConstructionScript
  (|CallParentFunction))

(fn GetDistanceforAttack
  (params (InAttackType :type AttackTypes_AI%20Enum :default "NewEnumerator5") (InDistanceToTarget :type Float%20%28double-precision%29))
  ;[1 1 1] If current attack min distance is less than distance to target do a jump
  (bind (_boutinrange _outdistance) (|CallParentFunction InAttackType InDistanceToTarget))
  (LocalVariables|SetTempDistance _outdistance)
  (bind _output_get (LocalVariables|SetbTempOutAttack _boutinrange))
  (if _output_get
    _
    (elif (and (Utilities|Enum|Equal(Enum) InAttackType "NewEnumerator2") (<= InDistanceToTarget (Utilities|Struct|BreakFloatRangeBound (Utilities|Struct|BreakFloatRange (LocalVariables|GetTempDistance)))))
      (if (not (Variables|/Game/UltimateCharacter/Blueprints/Characters/BaseCharacter_BP.BaseCharacter_BP_C|GetbIsLanded (Variables|Default|GetPawn_AI)))
        (return true (LocalVariables|GetTempDistance))
        (else
          (Default|OnStartJump (Variables|Default|GetPawn_AI))))))
  (return (LocalVariables|GetbTempOutAttack) (LocalVariables|GetTempDistance)))