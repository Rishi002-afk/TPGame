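; Base damage type for the UltimateCharacter system that describes how a hit affects a character.
; It holds a per-body-region damage multiplier struct for head, hand, body and leg, plus a can-kill setting and a camera shake.
; Simple getter functions expose each value, with no other logic in the graphs.
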(fn GetHeadDamageModifier
  (return (Utilities|Struct|BreakFDamageModifiers (Variables|UltimateCharacter|GetDamageModifier))))

(fn GetHandDamageModifier
  (return (Utilities|Struct|BreakFDamageModifiers (Variables|UltimateCharacter|GetDamageModifier))))

(fn GetBodyDamageModifier
  (return (Utilities|Struct|BreakFDamageModifiers (Variables|UltimateCharacter|GetDamageModifier))))

(fn GetLegDamageModifier
  (return (Utilities|Struct|BreakFDamageModifiers (Variables|UltimateCharacter|GetDamageModifier))))

(fn GetCanKill
  (return (Variables|UltimateCharacter|GetbCanKill)))

(fn GetCameraShake
  (return (Variables|UltimateCharacter|GetCameraShake)))