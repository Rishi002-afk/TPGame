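; PlayerState Blueprint that stores the player's team number and exposes a setter and getter for it.
; TeamNumber has a RepNotify that only writes a debug message on non-authority instances, and the setter logs the new value.
; Logging goes through a DebugMessage wrapper that forwards when the ShowDebugMessage flag is on or the message is of one specific type.
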(event EventBeginPlay)

(event EventTick
  (params (DeltaSeconds :type Float%20%28single-precision%29)))

(fn ConstructionScript)

(fn SetTeamNumber
  (params (InTeam :type Integer))
  (bind _output_get (Variables|Internal|SetTeamNumber InTeam))
  (Debug|DebugMessage "PlayerState_BP" "SetTeamNumber" (Utilities|String|ToString(Integer) _output_get) "NewEnumerator0"))

(fn OnRepTeamNumber
  (if (not (Utilities|Enum|Equal(Enum) (Networking|GetLocalRole) "ROLE_Authority"))
    (Debug|DebugMessage "PlayerState_BP" "OnRepTeamNumber" "" "NewEnumerator0")))

(fn DebugMessage
  (params (InCallerName :type String) (InFunction :type String) (InMessage :type String) (InMessageType :type MessageType%20Enum :default "NewEnumerator0"))
  (if (or (Variables|Debug|GetbShowDebugMessage) (Utilities|Enum|Equal(Enum) InMessageType "NewEnumerator3"))
    (CallFunction|ShowDebugMessage InCallerName InFunction InMessage InMessageType)))

(fn GetTeamNumber
  (return (Variables|Internal|GetTeamNumber)))