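; Explosion effect actor that plays surface-specific particles and sound at its location, then removes itself.
; On BeginPlay, GetEffectInfo maps the hit's physical surface type to an effect set, falling back to a default.
; It also attaches a randomly rolled decal to the hit component, aligned to the impact normal.
; Tick repeatedly scales down the explosion light's intensity and destroys the actor when the fade-out time elapses.
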(event EventBeginPlay
  (bind _decal (Variables|UltimateCharacter-Effects|GetDecal))
  (bind _surfacehit (Variables|Surface|GetSurfaceHit))
  (bind (_decalmaterial _decalsize _lifespan) (Utilities|Struct|BreakDecalData _decal))
  (bind (_bblockinghit _binitialoverlap _time _distance _location _impactpoint _normal _impactnormal _physmat _hitactor _hitcomponent _hitbonename) (Collision|BreakHitResult _surfacehit))
  (bind _returnvalue (Math|Conversions|RotationFromXVector _impactnormal))
  (Utilities|FlowControl|Sequence
    (:then_0
      ;[1 1 1] Find effect for the surface
      (bind _outeffect (CallFunction|GetEffectInfo))
      (Variables|Internal|SetExplosionFX (.Effect (Utilities|Struct|BreakHitEffect_Info _outeffect)))
      (Variables|Internal|SetExplosionSound (.Sound (Utilities|Struct|BreakHitEffect_Info _outeffect))))
    (:then_1
      ;[1 1 1] Spawn explosion effect
      (Utilities|IsValid (Variables|Internal|GetExplosionFX)
        (:Is%20Valid
          (Effects|SpawnEmitteratLocation (Variables|Internal|GetExplosionFX) (Transformation|GetActorLocation) (Transformation|GetActorRotation) (Variables|UltimateCharacter-Effects|GetEffectScale)))))
    (:then_2
      ;[1 1 1] Spawn sound at explosion location
      (Utilities|IsValid (Variables|Internal|GetExplosionSound)
        (:Is%20Valid
          (Audio|PlaySoundatLocation (Variables|Internal|GetExplosionSound) (Transformation|GetActorLocation) "0, 0, 0" 1.0 1.0 0.0 0 0 0))))
    (:then_3
      ;[1 1 1] Spawn decal for the explosion
      (Utilities|IsValid _decalmaterial
        (:Is%20Valid
          (Class|GameplayStatics|SpawnDecalAttached _decalmaterial (Math|Vector|MakeVector _decalsize _decalsize 1.0) _hitcomponent _hitbonename _impactpoint (Math|Rotator|MakeRotator (Math|Random|RandomFloatinRange -1.8e+02 1.8e+02) (.pitch _returnvalue) (.yaw _returnvalue)) "KeepWorldPosition" _lifespan))))))

(event EventTick
  (params (DeltaSeconds :type Float%20%28single-precision%29))
  (bind _returnvalue (Actor|GetGameTimeSinceCreation))
  (bind _explosionlightfadeout (Variables|UltimateCharacter-Effects|GetExplosionLightFadeOut))
  (bind _explosionlight (Variables|Default|GetExplosionLight))
  (bind _returnvalue_2 (- _explosionlightfadeout _returnvalue))
  (bind _returnvalue_3 (Math|Float|Max(Float) 0.0 _returnvalue_2))
  ;[1 1 1] Fading light to zero
  (if (> _returnvalue_3 0.0)
    (Rendering|Components|Light|SetIntensity _explosionlight (* (Variables|/Script/Engine.LightComponentBase|GetIntensity _explosionlight) (- 1.0 (Math|Float|Square (/ _returnvalue_3 (Variables|UltimateCharacter-Effects|GetExplosionLightFadeOut))))))
    (else
      (Actor|DestroyActor))))

(fn ConstructionScript)

(fn GetEffectInfo
  (bind _hiteffects (Variables|UltimateCharacter-Effects|GetHitEffects))
  (bind _surfacehit (Variables|Surface|GetSurfaceHit))
  (bind (_default _water _wood _flesh _glass _stone _metal) (Utilities|Struct|BreakHitEffects_Info _hiteffects))
  (bind _physmat (Collision|BreakHitResult _surfacehit))
  (Utilities|IsValid _physmat
    (:Is%20Valid
      (switch Utilities|FlowControl|Switch|SwitchonEPhysicalSurface (Variables|/Script/Engine.PhysicalMaterial|GetSurfaceType _physmat)
        (:SurfaceType_Default
          (LocalVariables|SetTempHitEffect _default :!label _label))
        (:SurfaceType1
          (LocalVariables|SetTempHitEffect _water))
        (:SurfaceType2
          (LocalVariables|SetTempHitEffect _wood))
        (:SurfaceType3
          (LocalVariables|SetTempHitEffect _flesh))
        (:SurfaceType4
          (LocalVariables|SetTempHitEffect _glass))
        (:SurfaceType5
          (LocalVariables|SetTempHitEffect _stone))
        (:SurfaceType6
          (LocalVariables|SetTempHitEffect _metal))))
    (:Is%20Not%20Valid
      (goto _label)))
  (return (LocalVariables|GetTempHitEffect)))