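; ImpactEffect_BP is an impact effect actor that plays surface-specific feedback for a hit when it begins play.
; GetImpactFX maps the physical material's surface type from SurfaceHit to a particle and sound, covering materials and body parts with a default fallback.
; It spawns both at the actor's location, then attaches a timed decal to the hit component and bone, aligned to the normal with random roll.
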(event EventBeginPlay
  (bind _surfacehit (Variables|Internal|GetSurfaceHit))
  (bind _decal (Variables|UltimateCharacter-Effects|GetDecal))
  (bind (_decalmaterial _decalsize _lifespan) (Utilities|Struct|BreakDecalData _decal))
  (bind (_bblockinghit _binitialoverlap _time _distance _location _impactpoint _normal _impactnormal _physmat _hitactor _hitcomponent _hitbonename) (Collision|BreakHitResult _surfacehit))
  (bind _returnvalue (Math|Conversions|RotationFromXVector _impactnormal))
  (bind (_outparticle _outsound) (CallFunction|GetImpactFX (select (== _physmat 0) "SurfaceType_Default" (Variables|/Script/Engine.PhysicalMaterial|GetSurfaceType _physmat))))
  (Utilities|FlowControl|Sequence
    (:then_0
      (Utilities|IsValid _outparticle
        (:Is%20Valid
          (Effects|SpawnEmitteratLocation _outparticle (Transformation|GetActorLocation)))))
    (:then_1
      (Utilities|IsValid _outsound
        (:Is%20Valid
          (Audio|PlaySoundatLocation _outsound (Transformation|GetActorLocation) "0, 0, 0" 1.0 1.0 0.0 0 0 0))))
    (:then_2
      (Utilities|IsValid _decalmaterial
        (:Is%20Valid
          (Class|GameplayStatics|SpawnDecalAttached _decalmaterial (Math|Vector|MakeVector _decalsize _decalsize 1.0) _hitcomponent _hitbonename _impactpoint (Math|Rotator|MakeRotator (Math|Random|RandomFloatinRange -1.8e+02 1.8e+02) (.pitch _returnvalue) (.yaw _returnvalue)) "KeepWorldPosition" _lifespan))))))

(fn ConstructionScript)

(fn GetImpactFX
  (params (InSurface :type EPhysicalSurface%20Enum :default "SurfaceType_Default"))
  (bind _fx (Variables|UltimateCharacter-Effects|GetFX))
  (bind (_default _water _wood _flesh _glass _stone _metal _head _body _hand _leg) (Utilities|Struct|BreakHitEffects_Info _fx))
  (bind (_effect _sound) (Utilities|Struct|BreakHitEffect_Info _leg))
  (bind (_effect_2 _sound_2) (Utilities|Struct|BreakHitEffect_Info _body))
  (bind (_effect_3 _sound_3) (Utilities|Struct|BreakHitEffect_Info _hand))
  (bind (_effect_4 _sound_4) (Utilities|Struct|BreakHitEffect_Info _default))
  (bind (_effect_5 _sound_5) (Utilities|Struct|BreakHitEffect_Info _water))
  (bind (_effect_6 _sound_6) (Utilities|Struct|BreakHitEffect_Info _wood))
  (bind (_effect_7 _sound_7) (Utilities|Struct|BreakHitEffect_Info _flesh))
  (bind (_effect_8 _sound_8) (Utilities|Struct|BreakHitEffect_Info _glass))
  (bind (_effect_9 _sound_9) (Utilities|Struct|BreakHitEffect_Info _stone))
  (bind (_effect_10 _sound_10) (Utilities|Struct|BreakHitEffect_Info _metal))
  (bind (_effect_11 _sound_11) (Utilities|Struct|BreakHitEffect_Info _head))
  (switch Utilities|FlowControl|Switch|SwitchonEPhysicalSurface InSurface
    (:SurfaceType_Default
      (return _effect_4 _sound_4))
    (:SurfaceType1
      (return _effect_5 _sound_5))
    (:SurfaceType2
      (return _effect_6 _sound_6))
    (:SurfaceType3
      (return _effect_7 _sound_7))
    (:SurfaceType4
      (return _effect_8 _sound_8))
    (:SurfaceType5
      (return _effect_9 _sound_9))
    (:SurfaceType6
      (return _effect_10 _sound_10))
    (:SurfaceType7
      (return _effect_11 _sound_11))
    (:SurfaceType8
      (return _effect_2 _sound_2))
    (:SurfaceType9
      (return _effect_3 _sound_3))
    (:SurfaceType10
      (return _effect _sound))))