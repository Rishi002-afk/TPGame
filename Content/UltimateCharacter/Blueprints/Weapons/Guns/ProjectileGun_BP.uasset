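; ProjectileGun_BP is a gun Blueprint that fires projectile actors rather than setting up any hit logic itself.
; FireWeapon calls InternalFireWeapon, which passes the muzzle location and the owning pawn's control rotation to ServerFireProjectile.
; That event spawns ProjectileClass with the gun as owner, then calls InitVelocity on the projectile to launch it.
; BeginPlay sets the weapon type, and both firing steps emit debug messages.
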(event Custom|ServerFireProjectile
  (params (InOrigin :type Vector) (InShootDir :type Rotator))
  (CallFunction|ShowDebugMessage "ProjectileGun_BP" "ServerFireProjectile" (Utilities|String|Append (Utilities|String|ToString(Name) (Variables|Default|GetWeaponTag)) " spawning projectile.") "NewEnumerator0")
  ;[1 1 1] Spawning projectile & init velocity of projectile
  (bind _returnvalue (Game|SpawnActorfromClass (Variables|UltimateCharacter|GetProjectileClass) (Math|Transform|MakeTransform InOrigin InShootDir) "Undefined" "SelectDefaultAtRuntime" self (Variables|Default|GetInstigator)))
  (Utilities|IsValid _returnvalue
    (:Is%20Valid
      (Default|InitVelocity _returnvalue))))

(event EventBeginPlay
  (|CallParentFunction)
  (Variables|Default|SetWeaponType "NewEnumerator2"))

(event Collision|EventActorBeginOverlap
  (params (OtherActor :type Actor%20Object%20Reference))
  (|CallParentFunction OtherActor) ; This node is disabled and will not be called.\nDrag off pins to build functionality.
)

(event EventTick
  (params (DeltaSeconds :type Float%20%28single-precision%29))
  (|CallParentFunction DeltaSeconds) ; This node is disabled and will not be called.\nDrag off pins to build functionality.
)

(event EventFireWeapon
  (Weapon|InternalFireWeapon))

(fn ConstructionScript
  (|CallParentFunction))

(fn InternalFireWeapon
  (CallFunction|ShowDebugMessage "ProjectileGun_BP" "InternalFireWeapon" (Utilities|String|ToString(Name) (Variables|Default|GetWeaponTag)) "NewEnumerator0")
  (bind _output_get (LocalVariables|SetTempOrigin (CallFunction|GetStartFireLocation(Muzzle))))
  (CallFunction|ServerFireProjectile _output_get (Pawn|GetControlRotation (Variables|Default|GetMyPawn) :!class /Script/Engine.Pawn)))