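; Base item for bombard attacks: a non-respawning pickup that takes its tag from the BombardClass defaults.
; Pickup looks up T_Player_Bombard by character plus item tag, then creates and initializes the player's attack item with UI, animation, camera and cursor.
; Use spawns Count bombards at the instigator, attaching them to the mesh socket unless they spawn at target location.
; Spawned bombards are tracked in Attacks and disabled when the item is destroyed.
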(event EventBeginPlay
  ;[1 1 1] Set item tag, and don't allow respawn
  (Variables|Default|SetItemTag (.ItemTag (Utilities|GetClassDefaults (Variables|UltimateCharacter|GetBombardClass))))
  (|CallParentFunction)
  (Variables|Default|SetbAllowRespawn false))

(event Collision|EventActorBeginOverlap
  (params (OtherActor :type Actor%20Object%20Reference))
  (|CallParentFunction OtherActor) ; This node is disabled and will not be called.\nDrag off pins to build functionality.
)

(event EventTick
  (params (DeltaSeconds :type Float%20%28single-precision%29))
  (|CallParentFunction DeltaSeconds) ; This node is disabled and will not be called.\nDrag off pins to build functionality.
)

(event EventUse
  ;[1 1 1] Override base functions
  (|CallParentFunction)
  (Interact|UseOverride))

(event EventDestroyed
  ;[1 1 1] Override base functions
  (|CallParentFunction)
  (Internal|DisableBomards))

(fn ConstructionScript
  (|CallParentFunction)
  (Variables|Default|SetItemType "NewEnumerator1"))

(fn UseOverride
  (bind _returnvalue (Game|GetInstigator))
  (bind _itemconfig (Variables|Default|GetItemConfig))
  (bind (_inventoryattachsocket _difficultymultiplier) (Utilities|Struct|BreakT_AttackItem_Struct _itemconfig))
  (CallFunction|DebugMessage "Base_Bombard_Pickup_BP" "UseOverride" (Utilities|String|ToString(Name) (Variables|Default|GetItemTag)) "NewEnumerator0")
  (for _index (range 0 (- (Variables|Default|GetCount) 1))
    ;[1 1 1] Spawn & store bombard actor
    (bind _returnvalue_2 (Game|SpawnActorfromClass (Variables|UltimateCharacter|GetBombardClass) (Math|Transform|MakeTransform (Transformation|GetActorLocation _returnvalue)) "AlwaysSpawn" "SelectDefaultAtRuntime" 0 (Variables|Internal|GetInterval) _returnvalue))
    (bind _output_get (LocalVariables|SetTempBombard _returnvalue_2))
    (Variables|/Game/UltimateCharacter/Blueprints/Weapons/Bombards/BaseBombard_BP.BaseBombard_BP_C|SetDifficultyMultiplier _output_get _difficultymultiplier)
    (if (Variables|/Game/UltimateCharacter/Blueprints/Weapons/Bombards/BaseBombard_BP.BaseBombard_BP_C|GetbSpawnAtTargetLocation _output_get)
      _
      (else
        (Transformation|AttachComponentToComponent (LocalVariables|GetTempBombard) (Variables|Character|GetMesh) (Utilities|Array|Get(acopy) _inventoryattachsocket) "SnapToTarget" "SnapToTarget" "KeepWorld" true)))
    (Utilities|Array|Add (Variables|Internal|GetAttacks) (LocalVariables|GetTempBombard)))
  (Variables|Default|SetCount 0))

(fn DisableBomards
  (CallFunction|DebugMessage "Base_Bombard_Pickup_BP" "DisableBombard" (Utilities|String|ToString(Name) (Variables|Default|GetItemTag)) "NewEnumerator0")
  ;[1 1 1] Try to remove & disable spawned bombards
  (for _array_element (Variables|Internal|GetAttacks)
    (Utilities|IsValid _array_element
      (:Is%20Valid
        (Default|DisableBombard _array_element))
      (:Is%20Not%20Valid
        _))
    (Utilities|Array|RemoveItem (Variables|Internal|GetAttacks) _array_element)))

(fn SetInterval
  (params (InInterval :type Float%20%28double-precision%29))
  (CallFunction|DebugMessage "Base_BombardItem_BP" "SetInterval" (Utilities|String|ToString(Name) (Variables|Default|GetItemTag)) "NewEnumerator0")
  (Variables|Internal|SetInterval InInterval))

(fn HasValidClass
  (return (Utilities|IsValidClass (Variables|UltimateCharacter|GetBombardClass))))

(fn PickupItemforPlayer
  (bind _itemtag (Variables|Default|GetItemTag))
  (bind _charactertarget (Variables|Default|GetCharacterTarget))
  (bind _bombardsinventory (Variables|/Game/UltimateCharacter/Blueprints/Characters/BaseCharacter_BP.BaseCharacter_BP_C|GetBombardsInventory _charactertarget))
  (bind (_value _returnvalue) (Utilities|Map|Find _bombardsinventory _itemtag))
  (CallFunction|DebugMessage "Base_Bombard_Pickup_BP" "PickupItemForPlayer" (Utilities|String|ToString(Name) (Variables|Default|GetItemTag)) "NewEnumerator0")
  (Utilities|IsValid (Variables|Default|GetCharacterTarget)
    (:Is%20Valid
      ;[1 1 1] Find from table
      (bind _returnvalue_2 (Utilities|GetDataTableRow "/Game/UltimateCharacter/Blueprints/Data/Tables/Player/T_Player_Bombard.T_Player_Bombard" (Utilities|String|StringToName (Utilities|String|Append (Utilities|String|ToString(Name) (Variables|/Game/UltimateCharacter/Blueprints/Characters/BaseCharacter_BP.BaseCharacter_BP_C|GetCharacterTag (Variables|Default|GetCharacterTarget))) (Utilities|String|ToString(Name) (Variables|Default|GetItemTag)))))
        (:then
          ;[1 1 1] Spawn bombards & initialize for player
          (bind _outitemindex (Default|SpawnAttackItems (Variables|Default|GetCharacterTarget) (Utilities|Struct|BreakT_Bombard_Struct (.Base (Utilities|Struct|BreakT_PlayerBombard_Struct _returnvalue_2))) (select _returnvalue _value (Utilities|Map|Length _bombardsinventory)) (Variables|Default|GetItemTag) (Utilities|GetClass self)))
          (LocalVariables|SetTempOutIndex _outitemindex)
          (if (> (LocalVariables|GetTempOutIndex) -1)
            (Default|InitializeforPlayer (Utilities|Array|Get(acopy) (Variables|/Game/UltimateCharacter/Blueprints/Characters/BaseCharacter_BP.BaseCharacter_BP_C|GetAttackItems (Variables|Default|GetCharacterTarget)) (LocalVariables|GetTempOutIndex)) (.UIConfig (Utilities|Struct|BreakT_PlayerBombard_Struct _returnvalue_2)) (.FirstPersonAnimation (Utilities|Struct|BreakT_PlayerBombard_Struct _returnvalue_2)) (.CameraConfig (Utilities|Struct|BreakT_PlayerBombard_Struct _returnvalue_2)))
            (bind _asplayer_character_bp (Utilities|Casting|CastToPlayerCharacter_BP (Variables|Default|GetCharacterTarget))
              (:then
                (Default|SpawnCursor _asplayer_character_bp (Utilities|Struct|BreakT_PlayerCamera_Struct (.CameraConfig (Utilities|Struct|BreakT_PlayerBombard_Struct _returnvalue_2))) false))
              (:CastFailed
                _))
            (return true)
            (else
              (CallFunction|DebugMessage "Base_Bombard_Pickup_BP" "PickupItemForPlayer" (Utilities|String|Append (Utilities|String|ToString(Name) (Variables|Default|GetItemTag)) " Failed, index is not valid.") "NewEnumerator2")
              (return false))))
        (:RowNotFound
          (CallFunction|DebugMessage "Base_Bombard_Pickup_BP" "PickupItemForPlayer" (Utilities|String|Append (Utilities|String|ToString(Name) (Variables|Default|GetItemTag)) " not found in table") "NewEnumerator2")
          (Default|HUDMessage (Variables|Default|GetCharacterTarget) "You're not allowed to pickup the item" "NewEnumerator2")
          (return false))))
    (:Is%20Not%20Valid
      (CallFunction|DebugMessage "Base_Bombard_Pickup_BP" "PickupItemForPlayer" "Character target is not valid!" "NewEnumerator2")
      (return false))))