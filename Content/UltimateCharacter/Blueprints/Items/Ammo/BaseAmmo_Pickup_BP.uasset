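; Base ammo pickup item that refills a compatible gun in the character's inventory and registers as an AI sight stimulus.
; On pickup, GiveAmmo finds the first gun matching GunTypes, by class or parent class, that is below max ammo.
; It adds AmmoClips worth of that gun's clip size and runs the parent pickup only on success, otherwise shows a HUD message.
; Overlap-based pickup is left unconnected.
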(event OnComponentBeginOverlap(Mesh)
  (params (OverlappedComponent :type Primitive%20Component%20Object%20Reference) (OtherActor :type Actor%20Object%20Reference) (OtherComp :type Primitive%20Component%20Object%20Reference) (OtherBodyIndex :type Integer) (bFromSweep :type Boolean) (SweepResult :type Hit%20Result%20Structure%20%28by%20ref%29))
  ;[1 1 1] Overlap pickup is not activated you can activate by connecting nodes
)

(event EventBeginPlay
  (|CallParentFunction)
  (Class|AIPerceptionSystem|RegisterPerceptionStimuliSource "/Script/AIModule.AISense_Sight" self))

(event Collision|EventActorBeginOverlap
  (params (OtherActor :type Actor%20Object%20Reference))
  (|CallParentFunction OtherActor) ; This node is disabled and will not be called.\nDrag off pins to build functionality.
)

(event EventTick
  (params (DeltaSeconds :type Float%20%28single-precision%29))
  (|CallParentFunction DeltaSeconds) ; This node is disabled and will not be called.\nDrag off pins to build functionality.
)

(event EventOnPickup
  (params (InCharacter :type Base%20Character%20BP%20Object%20Reference))
  ;[1 1 1] Pickup item when pickup command received
  (bind _output_get (Variables|Internal|SetCharacterTarget InCharacter))
  (Utilities|IsValid _output_get
    (:Is%20Valid
      (bind _boutgave (Gun|GiveAmmo (Variables|Internal|GetCharacterTarget)))
      (if _boutgave
        (|CallParentFunction (Variables|Internal|GetCharacterTarget))))
    (:Is%20Not%20Valid
      (CallFunction|DebugMessage "BaseAmmo_Pickup_BP" "OnPickup" (Utilities|String|Append "Character is not valid to pickup " (Utilities|GetDisplayName self)) "NewEnumerator0"))))

(fn ConstructionScript
  (|CallParentFunction))

(fn IsforGun
  (params (InGun :type Base%20Gun%20BP%20Class%20Reference))
  (CallFunction|DebugMessage "BaseAmmo_Pickup_BP" "IsForGun" (Utilities|String|ToString(Name) (Variables|Default|GetItemTag)) "NewEnumerator0")
  ;[1 1 1] Check supported gun list
  (bind _array_element (Utilities|Array|ForEachLoopwithBreak (Variables|UltimateCharacter|GetGunTypes) :!label _label)
    (:LoopBody
      (if (or (Utilities|ClassIsChildOf InGun _array_element) (== _array_element InGun))
        (LocalVariables|SetbFound true)
        (goto _label Break)))
    (:Completed
      (return (LocalVariables|GetbFound)))))

(fn GiveAmmo
  (params (InCharacter :type Base%20Character%20BP%20Object%20Reference))
  (CallFunction|DebugMessage "BaseAmmo_Pickup_BP" "GiveAmmo" (Utilities|String|ToString(Name) (Variables|Default|GetItemTag)) "NewEnumerator0")
  ;[1 1 1] Check if character has compatible gun for this ammo
  (bind _array_element (Utilities|Array|ForEachLoopwithBreak (Variables|/Game/UltimateCharacter/Blueprints/Characters/BaseCharacter_BP.BaseCharacter_BP_C|GetInventory InCharacter) :!label _label)
    (:LoopBody
      (bind _asbase_gun_bp (Utilities|Casting|CastToBaseGun_BPClass (Utilities|GetClass _array_element)))
      (if (Gun|IsforGun _asbase_gun_bp)
        (bind _output_get (LocalVariables|SetTempWeapon _array_element))
        (if (< (Default|GetCurrentAmmo _output_get) (Default|GetMaxAmmo _output_get))
          (LocalVariables|SetbTempGiveAmmo true)
          (goto _label Break))))
    (:Completed
      (if (LocalVariables|GetbTempGiveAmmo)
        (Default|GiveAmmo (LocalVariables|GetTempWeapon) (* (Default|GetAmmoPerClip (LocalVariables|GetTempWeapon)) (Variables|UltimateCharacter|GetAmmoClips)))
        (return true)
        (else
          (CallFunction|DebugMessage "BaseAmmo_Pickup_BP" "GiveAmmo" "Character has not weapon in inventory or weapon is full" "NewEnumerator1")
          (Default|HUDMessage InCharacter "You don't have any supported weapon for this ammo." "NewEnumerator1")
          (return false))))))