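; Base summon item that spawns AI allies for its user, taking its tag from the AI class defaults.
; Use spawns Count characters at navigable points ahead of the instigator, assigning team and fast target recognition via blackboard.
; Summons copy an AI owner's target or bind to a player owner to die with them.
; Player pickup requires a T_Player_Summon row keyed by character and item tags; deletion skips items marked -1 in SummonInventory.
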(event EventBeginPlay
  (Variables|Default|SetItemTag (.CharacterTag (Utilities|GetClassDefaults (Variables|UltimateCharacter|GetAICharacterClass))))
  (|CallParentFunction)
  (Variables|Default|SetbAllowRespawn false))

(event Collision|EventActorBeginOverlap
  (params (OtherActor :type Actor%20Object%20Reference))
  (|CallParentFunction OtherActor) ; This node is disabled and will not be called.\nDrag off pins to build functionality.
)

(event EventTick
  (params (DeltaSeconds :type Float%20%28single-precision%29))
  (|CallParentFunction DeltaSeconds) ; This node is disabled and will not be called.\nDrag off pins to build functionality.
)

(event EventUse
  (|CallParentFunction)
  (CallFunction|UseOverride))

(event EventDeleteItem
  (bind _returnvalue (Game|GetInstigator))
  ;[1 1 1] Don't need to delete unlimit reusable attack items, for example narbash can throw his mace unlimited
  (Utilities|IsValid _returnvalue
    (:Is%20Valid
      (bind _asbase_character_bp (Utilities|Casting|CastToBaseCharacter_BP _returnvalue)
        (:then
          (if (.ReturnValue (Utilities|Map|Find (Variables|/Game/UltimateCharacter/Blueprints/Characters/BaseCharacter_BP.BaseCharacter_BP_C|GetSummonInventory _asbase_character_bp) (Variables|Default|GetItemTag)))
            (if (!= (.Value (Utilities|Map|Find (Variables|/Game/UltimateCharacter/Blueprints/Characters/BaseCharacter_BP.BaseCharacter_BP_C|GetSummonInventory _asbase_character_bp) (Variables|Default|GetItemTag))) -1)
              (|CallParentFunction))
            (else
              (|CallParentFunction))))
        (:CastFailed
          (|CallParentFunction))))
    (:Is%20Not%20Valid
      (|CallParentFunction))))

(fn ConstructionScript
  (|CallParentFunction)
  (Variables|Default|SetItemType "NewEnumerator2"))

(fn UseOverride
  (bind _returnvalue (Game|GetInstigator))
  (CallFunction|DebugMessage "Base_SummonItem_BP" "UseOverride" (Utilities|String|ToString(Name) (Variables|Default|GetItemTag)) "NewEnumerator0")
  ;[1 1 1] Spawn & set character rotation same as owner
  (LocalVariables|SetTempCharacterRotation (Pawn|GetControlRotation _returnvalue :!class /Script/Engine.Pawn))
  (for _index (range 0 (- (Variables|Default|GetCount) 1))
    (bind _randomlocation (Class|NavigationSystemV1|GetRandomLocationinNavigableRadius (+ (+ (Transformation|GetActorLocation _returnvalue) (* (Transformation|GetActorForwardVector _returnvalue) 2.5e+02)) "0, 0,150.000000") 1.5e+02 0 0))
    (bind _returnvalue_2 (Game|SpawnActorfromClass (Variables|UltimateCharacter|GetAICharacterClass) (Math|Transform|MakeTransform _randomlocation (LocalVariables|GetTempCharacterRotation)) "Undefined" "SelectDefaultAtRuntime" 0 0 (Game|GetInstigator)))
    (LocalVariables|SetTempCharacter _returnvalue_2)
    ;[1 1 1] Assign team number
    (bind _asaicontroller_bp (Utilities|Casting|CastToAIController_BP (Pawn|GetController (LocalVariables|GetTempCharacter)))
      (:then
        (LocalVariables|SetTempController _asaicontroller_bp)
        (Default|UpdateTeamNumber (LocalVariables|GetTempController) (Variables|Internal|GetTeamNumber))
        (Utilities|IsValid (AI|GetBlackboard (LocalVariables|GetTempController))
          (:Is%20Valid
            (Utilities|FlowControl|Sequence
              (:then_0
                ;[1 1 1] Try to get target from the owner
                (bind _asaicharacter_bp (Utilities|Casting|CastToAICharacter_BP (Game|GetInstigator)))
                (bind _asbase_character_bp (Utilities|Casting|CastToBaseCharacter_BP (AI|Components|Blackboard|GetValueasObject (AI|GetBlackboard (Pawn|GetController _asaicharacter_bp)) (Utilities|Name|MakeLiteralName "Target"))))
                ;[1 1 1] Set target manually for spawned character also set recognize remaining time very small amount
                (AI|Components|Blackboard|SetValueasObject (AI|GetBlackboard (LocalVariables|GetTempController)) (Utilities|Name|MakeLiteralName "Target") _asbase_character_bp))
              (:then_1
                ;[1 1 1] New summoned character must recognize his target very fast
                (AI|Components|Blackboard|SetValueasFloat (AI|GetBlackboard (LocalVariables|GetTempController)) (Utilities|Name|MakeLiteralName "RemainRecognizeTime") 0.1))
              (:then_2
                ;[1 1 1] Bind spawned AI character to the player owner to kill the AI character after dying the player
                (bind _asplayer_character_bp (Utilities|Casting|CastToPlayerCharacter_BP (Game|GetInstigator)))
                (Default|BindtoPlayerCharacter (LocalVariables|GetTempCharacter) _asplayer_character_bp))))
          (:Is%20Not%20Valid
            (CallFunction|DebugMessage "Base_SummonItem_BP" "UseOverride" (Utilities|String|Append "Blackboard is not valid for " (Utilities|String|ToString(Name) (Variables|Default|GetItemTag))) "NewEnumerator2"))))
      (:CastFailed
        (CallFunction|DebugMessage "Base_SummonItem_BP" "UseOverride" (Utilities|String|Append "Cast to BaseAIController_BP failed! " (Utilities|String|ToString(Name) (Variables|Default|GetItemTag)) " is in default team zero.") "NewEnumerator0"))))
  (Variables|Default|SetCount 0))

(fn HasValidClass
  (return (Utilities|IsValidClass (Variables|UltimateCharacter|GetAICharacterClass))))

(fn PickupItemforPlayer
  (bind _itemtag (Variables|Default|GetItemTag))
  (bind _charactertarget (Variables|Default|GetCharacterTarget))
  (bind _summoninventory (Variables|/Game/UltimateCharacter/Blueprints/Characters/BaseCharacter_BP.BaseCharacter_BP_C|GetSummonInventory _charactertarget))
  (bind (_value _returnvalue) (Utilities|Map|Find _summoninventory _itemtag))
  (CallFunction|DebugMessage "Base_SummonItem_BP" "PickupItemForPlayer" (Utilities|String|ToString(Name) (Variables|Default|GetItemTag)) "NewEnumerator0")
  (Utilities|IsValid (Variables|Default|GetCharacterTarget)
    (:Is%20Valid
      ;[1 1 1] Get item data for player from table
      (bind _returnvalue_2 (Utilities|GetDataTableRow "/Game/UltimateCharacter/Blueprints/Data/Tables/Player/T_Player_Summon.T_Player_Summon" (Utilities|String|StringToName (Utilities|String|Append (Utilities|String|ToString(Name) (Variables|/Game/UltimateCharacter/Blueprints/Characters/BaseCharacter_BP.BaseCharacter_BP_C|GetCharacterTag (Variables|Default|GetCharacterTarget))) (Utilities|String|ToString(Name) (Variables|Default|GetItemTag)))))
        (:then
          ;[1 1 1] Spawn & Initialize item for player
          (bind _outitemindex (Default|SpawnAttackItems (Variables|Default|GetCharacterTarget) (Utilities|Struct|BreakT_Summon_Struct (.Base (Utilities|Struct|BreakT_PlayerSummon_Struct _returnvalue_2))) (select _returnvalue _value (Utilities|Map|Length _summoninventory)) (Variables|Default|GetItemTag) (Utilities|GetClass self)))
          (LocalVariables|SetTempOutIndex _outitemindex)
          (if (> (LocalVariables|GetTempOutIndex) -1)
            (Default|InitializeforPlayer (Utilities|Array|Get(acopy) (Variables|/Game/UltimateCharacter/Blueprints/Characters/BaseCharacter_BP.BaseCharacter_BP_C|GetAttackItems (Variables|Default|GetCharacterTarget)) (LocalVariables|GetTempOutIndex)) (.UI (Utilities|Struct|BreakT_PlayerSummon_Struct _returnvalue_2)) (.FirstPersonAnimation (Utilities|Struct|BreakT_PlayerSummon_Struct _returnvalue_2)) (.CameraConfig (Utilities|Struct|BreakT_PlayerSummon_Struct _returnvalue_2)))
            (return true)
            (else
              (CallFunction|DebugMessage "Base_Bombard_Pickup_BP" "PickupItemForPlayer" (Utilities|String|Append (Utilities|String|ToString(Name) (Variables|Default|GetItemTag)) " Failed, index is not valid.") "NewEnumerator2")
              (return false))))
        (:RowNotFound
          (CallFunction|DebugMessage "Base_SummonItem_BP" "PickupItemForPlayer" (Utilities|String|Append (Utilities|String|ToString(Name) (Variables|Default|GetItemTag)) " not found in table") "NewEnumerator2")
          (Default|HUDMessage (Variables|Default|GetCharacterTarget) "You're not allowed to pickup summon items." "NewEnumerator2")
          (return false))))
    (:Is%20Not%20Valid
      (CallFunction|DebugMessage "Base_SummonItem_BP" "PickupItemForPlayer" "Character target is not valid!" "NewEnumerator2")
      (return false))))