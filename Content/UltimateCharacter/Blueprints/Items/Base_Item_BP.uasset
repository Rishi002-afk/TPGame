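; Base pickup item that characters can focus and pick up, highlighted through custom depth, with an empty Use function.
; BeginPlay briefly simulates physics for dropped or instigator-less items and activates the pickup.
; OnPickup makes noise, plays sound and effects, hides the mesh, then either starts a respawn timer or destroys the actor.
; An IsActive RepNotify mirrors picked-up and respawned visuals, rotation and collision on non-authority instances.
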(event EventBeginPlay
  (bind _mesh (Variables|Default|GetMesh))
  (Utilities|IsValid (Game|GetInstigator)
    (:Is%20Valid
      (if (Variables|Internal|GetbSpawnByDrop)
        (Physics|SetSimulatePhysics (Variables|Default|GetMesh) true :!label _label)
        (Transformation|SetActorRotation "0, 0, 0")
        (else
          ;[1 1 1] Makes mesh collision turn off to prevenet any unwanted collision to owner character
          (Collision|SetCollisionEnabled _mesh "NoCollision")
          (Collision|SetCollisionResponsetoAllChannels _mesh "ECR_Ignore"))))
    (:Is%20Not%20Valid
      (goto _label)))
  (Spawn|RespawnPickup)
  (Utilities|FlowControl|Delay 2.0)
  (Physics|SetSimulatePhysics (Variables|Default|GetMesh) false)
  (if (Variables|Internal|GetbSpawnByDrop)
    (Transformation|SetActorRotation "0, 0, 0")))

(event EventTick
  (params (DeltaSeconds :type Float%20%28single-precision%29)))

(fn ConstructionScript)

(fn OnBeginFocus
  ;[1 1 1] Set custom depth enable
  (Rendering|SetRenderCustomDepth (Variables|Default|GetMesh) true))

(fn OnEndFocus
  ;[1 1 1] Set custom depth disable when item is not in character focus
  (Rendering|SetRenderCustomDepth (Variables|Default|GetMesh) false))

(fn OnPickup
  (params (InCharacter :type Base%20Character%20BP%20Object%20Reference))
  (bind _pickupsound (Variables|UltimateCharacter|GetPickupSound))
  (bind (_sound _noise) (Utilities|Struct|BreakFBaseSound _pickupsound))
  (Debug|DebugMessage "Base_Pickup_BP" "OnPickup" (Utilities|String|Append (Utilities|String|ToString(Name) (Variables|Internal|GetItemTag)) " for " (Utilities|String|ToString(Name) (Variables|/Game/UltimateCharacter/Blueprints/Characters/BaseCharacter_BP.BaseCharacter_BP_C|GetCharacterTag InCharacter))) "NewEnumerator0")
  ;[1 1 1] Make noise
  (Default|MakePawnNoise InCharacter _noise)
  ;[1 1 1] Play pickup sound
  (Audio|PlaySoundatLocation _sound (Transformation|GetActorLocation) "0, 0, 0" 1.0 1.0 0.0 0 0 0)
  (Variables|Internal|SetbIsActive false)
  (Pickup|OnPickedUp)
  ;[1 1 1] Set timer to repspawn if we need
  (if (Variables|UltimateCharacter|GetbAllowRespawn)
    (Utilities|Time|SetTimerbyFunctionName self "RespawnPickup" (Variables|UltimateCharacter|GetRespawnTime))
    (else
      (Actor|DestroyActor))))

(fn RespawnPickup
  ;[1 1 1] Respawn pickup item
  (Debug|DebugMessage "Base_Pickup_BP" "RespawnPickup" (Utilities|String|ToString(Name) (Variables|Internal|GetItemTag)) "NewEnumerator0")
  (Variables|Internal|SetbIsActive true)
  (Spawn|OnRespawned))

(fn OnRespawned
  (Debug|DebugMessage "Base_Pickup_BP" "OnRespawned" (Utilities|String|ToString(Name) (Variables|Internal|GetItemTag)) "NewEnumerator0")
  (Components|Activation|Activate (Variables|Default|GetRotatingMovement) true)
  (Components|Activation|Activate (Variables|Default|GetMeshEffect) true)
  ;[1 1 1] Enable collision and show mesh of item
  (Utilities|IsValid (Variables|Default|GetMesh)
    (:Is%20Valid
      (Rendering|SetVisibility (Variables|Default|GetMesh) true false)
      (Collision|SetCollisionEnabled (Variables|Default|GetMesh) "QueryAndPhysics"))
    (:Is%20Not%20Valid
      (Debug|DebugMessage "Base_Pickup_BP" "RespawnPickup" (Utilities|String|Append "Mesh is not valid " (Utilities|String|ToString(Name) (Variables|Internal|GetItemTag))) "NewEnumerator1"))))

(fn DebugMessage
  (params (InCallerName :type String) (InFunction :type String) (InMessage :type String) (InMessageType :type MessageType%20Enum :default "NewEnumerator0"))
  (if (or (Variables|UltimateCharacter-Debug|GetbShowDebugMessage) (Utilities|Enum|Equal(Enum) InMessageType "NewEnumerator3"))
    (CallFunction|ShowDebugMessage InCallerName InFunction InMessage InMessageType)))

(fn OnPickedUp
  (Debug|DebugMessage "Base_Pickup_BP" "OnPickupedUp" (Utilities|String|ToString(Name) (Variables|Internal|GetItemTag)) "NewEnumerator0")
  ;[1 1 1] Spawn pickup effect
  (Effects|SpawnEmitteratLocation (Variables|UltimateCharacter|GetPickupEffect) (Transformation|GetActorLocation))
  (Components|Activation|Deactivate (Variables|Default|GetMeshEffect))
  (Components|Activation|Deactivate (Variables|Default|GetRotatingMovement))
  (Utilities|IsValid (Variables|Default|GetMesh)
    (:Is%20Valid
      ;[1 1 1] Makes mesh inactive
      (Rendering|SetVisibility (Variables|Default|GetMesh) false false)
      (Physics|SetSimulatePhysics (Variables|Default|GetMesh) false)
      (Collision|SetCollisionEnabled (Variables|Default|GetMesh) "NoCollision"))
    (:Is%20Not%20Valid
      (Debug|DebugMessage "Base_Pickup_BP" "RespawnPickup" (Utilities|String|Append "Mesh is not valid " (Utilities|String|ToString(Name) (Variables|Internal|GetItemTag))) "NewEnumerator1"))))

(fn OnRepBIsActive
  (Debug|DebugMessage "Base_Pickup_BP" "OnRespawned" (Utilities|String|ToString(Name) (Variables|Internal|GetItemTag)) "NewEnumerator0")
  (if (not (Utilities|Enum|Equal(Enum) (Networking|GetLocalRole) "ROLE_Authority"))
    (if (Variables|Internal|GetbIsActive)
      (Spawn|OnRespawned)
      (else
        (Pickup|OnPickedUp)))))

(fn Use)

(fn DisableCollisionandPhysics
  (Physics|SetSimulatePhysics (Variables|Default|GetMesh) false)
  (Collision|SetCollisionEnabled (Variables|Default|GetMesh) "NoCollision")
  (Collision|SetCollisionResponsetoAllChannels (Variables|Default|GetMesh) "ECR_Ignore"))