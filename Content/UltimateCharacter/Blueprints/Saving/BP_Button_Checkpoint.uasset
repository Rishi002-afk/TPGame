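; A checkpoint button actor that presses down when overlapped and plays a logo celebration effect when the checkpoint triggers.
; Trigger begin and end overlaps play and reverse a timeline that moves the button and fades its glow.
; The TriggerOverlap override defers to its parent and, on success, spawns a burst particle and runs a timeline that lifts, spins and recolors the logo.
; Dynamic material instances created in the construction script drive both glow effects.
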(event OnComponentBeginOverlap(Trigger)
  (params (OverlappedComponent :type Primitive%20Component%20Object%20Reference) (OtherActor :type Actor%20Object%20Reference) (OtherComp :type Primitive%20Component%20Object%20Reference) (OtherBodyIndex :type Integer) (bFromSweep :type Boolean) (SweepResult :type Hit%20Result%20Structure%20%28by%20ref%29))
  ;[1 1 1] Animate button
  (bind (_direction _press _glow) (Timeline|Press Play)
    (:Update
      (Transformation|SetRelativeLocation (Variables|Default|GetButton) (Math|Vector|MakeVector 0.0 0.0 _press) false false)
      (Rendering|Material|SetVectorParameterValue (Variables|Default|GetButton%20material) "Emissive" (Math|Color|Lerp(LinearColor) :B "(R=0.603828,G=0.327778,B=0.000000,A=1.000000)" :Alpha _glow) :!class /Script/Engine.MaterialInstanceDynamic))))

(event OnComponentEndOverlap(Trigger)
  (params (OverlappedComponent :type Primitive%20Component%20Object%20Reference) (OtherActor :type Actor%20Object%20Reference) (OtherComp :type Primitive%20Component%20Object%20Reference) (OtherBodyIndex :type Integer))
  ;[1 1 1] Animate button
  (bind (_direction _press _glow) (Timeline|Press Reverse)
    (:Update
      (Transformation|SetRelativeLocation (Variables|Default|GetButton) (Math|Vector|MakeVector 0.0 0.0 _press) false false)
      (Rendering|Material|SetVectorParameterValue (Variables|Default|GetButton%20material) "Emissive" (Math|Color|Lerp(LinearColor) :B "(R=0.603828,G=0.327778,B=0.000000,A=1.000000)" :Alpha _glow) :!class /Script/Engine.MaterialInstanceDynamic))))

(event Custom|CheckpointEffect
  (bind _logomaterial (Variables|Default|GetLogoMaterial))
  ;[1 1 1] Logo effect
  (Effects|SpawnEmitterAttached "/Game/UltimateCharacter/Effects/DemoRoom/P_Particle_Burst.P_Particle_Burst" (Variables|Default|GetLogo) "None" "0,15.000000, 0")
  (bind (_direction _rotation _height _color) (Timeline|Spin PlayFromStart)
    (:Update
      (Transformation|SetRelativeLocation (Variables|Default|GetLogo) (Math|Vector|Lerp(Vector) "0, 0,0.000000" "0, 0,50.000000" _height) false false)
      (Transformation|SetRelativeRotation (Variables|Default|GetLogoBase) (Math|Rotator|MakeRotator 0.0 0.0 _rotation) false false)
      (Rendering|Material|SetScalarParameterValue (Variables|Default|GetLogoMaterial) "Emissive multiply" (+ (* _height 25.0) 1.0) :!class /Script/Engine.MaterialInstanceDynamic)
      (Rendering|Material|SetVectorParameterValue _logomaterial "Color" (Math|Color|Lerp(LinearColor) "(R=0.020289,G=0.428691,B=1.000000,A=1.000000)" "(R=0.428691,G=1.000000,B=0.020289,A=1.000000)" _color) :!class /Script/Engine.MaterialInstanceDynamic)
      (Rendering|Material|SetVectorParameterValue _logomaterial "ColorBase" (Math|Color|Lerp(LinearColor) "(R=0.000000,G=0.188235,B=1.000000,A=1.000000)" "(R=0.188235,G=1.000000,B=0.000000,A=1.000000)" _color) :!class /Script/Engine.MaterialInstanceDynamic))))

(event EventBeginPlay
  (|CallParentFunction) ; This node is disabled and will not be called.\nDrag off pins to build functionality.
)

(event Collision|EventActorBeginOverlap
  (params (OtherActor :type Actor%20Object%20Reference))
  (|CallParentFunction OtherActor) ; This node is disabled and will not be called.\nDrag off pins to build functionality.
)

(event EventTick
  (params (DeltaSeconds :type Float%20%28single-precision%29))
  (|CallParentFunction DeltaSeconds) ; This node is disabled and will not be called.\nDrag off pins to build functionality.
)

(fn ConstructionScript
  (|CallParentFunction)
  (bind _returnvalue (Rendering|Material|CreateDynamicMaterialInstance (Variables|Default|GetButton) 0 0 "None" :!class /Script/Engine.PrimitiveComponent)) ; Make and apply a dynamic material instance for the button
  (Variables|Default|SetButton%20material _returnvalue) ; Set the material as a variable for animating
  (bind _returnvalue_2 (Rendering|Material|CreateDynamicMaterialInstance (Variables|Default|GetLogo) 0 0 "None" :!class /Script/Engine.PrimitiveComponent)) ; Make and apply a dynamic material instance for the button
  (Variables|Default|SetLogoMaterial _returnvalue_2))

(fn TriggerOverlap
  (params (InActor :type Actor%20Object%20Reference))
  (bind _bout (|CallParentFunction InActor))
  (if _bout
    (CallFunction|CheckpointEffect)
    (else
      (return false))))