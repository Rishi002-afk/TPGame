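; Base arrow projectile Blueprint that launches toward a target location and sticks to whatever actor it hits.
; FireArrow stores range and target, then derives launch speed from clamped target distance times a multiplier and solves the toss velocity with SuggestProjectileVelocity.
; Its mesh starts hidden and becomes visible on DisableandDestroy.
; Explode runs parent logic, then attaches the arrow to the hit actor and teleports it to the impact point.
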(event EventBeginPlay
  (|CallParentFunction)
  (Rendering|SetVisibility (Variables|Character|GetMesh) false false))

(event Collision|EventActorBeginOverlap
  (params (OtherActor :type Actor%20Object%20Reference))
  (|CallParentFunction OtherActor) ; This node is disabled and will not be called.\nDrag off pins to build functionality.
)

(event EventInitVelocity
  (CallFunction|InitVelocityOverride))

(event EventDisableandDestroy
  (|CallParentFunction)
  (Rendering|SetVisibility (Variables|Character|GetMesh) true false))

(event EventExplode
  (params (InHit :type Hit%20Result%20Structure))
  (bind (_bblockinghit _binitialoverlap _time _distance _location _impactpoint _normal _impactnormal _physmat _hitactor) (Collision|BreakHitResult InHit))
  (|CallParentFunction InHit)
  (Transformation|AttachActorToActor _hitactor "None" "SnapToTarget" "KeepWorld" "KeepWorld" false)
  (Transformation|SetActorLocation _impactpoint false true))

(fn ConstructionScript
  (|CallParentFunction))

(fn FireArrow
  (params (InMaxDistance :type Float%20%28single-precision%29) (InTarget :type Vector))
  (CallFunction|ShowDebugMessage "Base_Arrow_ProjectileBP" "FireArrow" "" "NewEnumerator0")
  (Variables|Internal|SetMaxDistance InMaxDistance)
  (Variables|Internal|SetTargetLocation InTarget)
  (CallFunction|InitVelocity))

(fn InitVelocityOverride
  (bind _projectilemovement (Variables|Default|GetProjectileMovement))
  (CallFunction|ShowDebugMessage "Base_Arrow_ProjectileBP" "InitVelocity_Override" "" "NewEnumerator0")
  (bind _output_get (Variables|/Script/Engine.ProjectileMovementComponent|SetInitialSpeed (Variables|Default|GetProjectileMovement) (* (Math|Float|Clamp(Float) (Math|Vector|VectorLength (- (Transformation|GetActorLocation) (Variables|Internal|GetTargetLocation))) 1e+03 1e+04) (Variables|Default|GetSpeedMultiplier))))
  (bind _tossvelocity (Class|GameplayStatics|BlueprintSuggestProjectileVelocity (Transformation|GetActorLocation) (Variables|Internal|GetTargetLocation) _output_get 0.0 "DoNotTrace" 0.0 false false))
  (Variables|/Script/Engine.MovementComponent|SetVelocity _projectilemovement _tossvelocity)
  (Components|Activation|Activate _projectilemovement true))