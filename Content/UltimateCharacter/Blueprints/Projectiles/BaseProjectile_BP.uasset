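; Base projectile actor for thrown and fired attacks, configured from ProjectileConfig, that explodes on stop or on destruction at end of lifespan.
; Launch velocity comes from the player's throw velocity or, for AI, a suggested toss toward the predicted target location.
; The authority applies radial damage, excluding characters that block, damages the hit character directly with block reduction, and spawns the effect.
; The Exploded rep notify re-runs Explode on clients when a short trace misses.
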(event OnProjectileStop(ProjectileMovement)
  (params (ImpactResult :type Hit%20Result%20Structure%20%28by%20ref%29))
  ;[1 1 1] Event runs when projectile hit something
  (Variables|Internal|SetHitResult ImpactResult)
  (if (and (Utilities|Enum|Equal(Enum) (Networking|GetLocalRole) "ROLE_Authority") (not (Variables|Internal|GetbExploded)))
    (Debug|ShowDebugMessage "BaseProjectile_BP" "OnStopProjectile" (Utilities|String|Append (Utilities|String|ToString(Name) (Utilities|Struct|BreakFProjectileWeaponData (Variables|UltimateCharacter|GetProjectileConfig))) " stopped by " (Utilities|GetDisplayName (.HitActor (Collision|BreakHitResult (Variables|Internal|GetHitResult))))) "NewEnumerator0")
    (Explosion|Explode (Variables|Internal|GetHitResult))
    (Explosion|DisableandDestroy)))

(event EventBeginPlay
  ;[1 1 1] Initialize projectile at begining
  (Initialize|Initialize))

(event Collision|EventActorBeginOverlap
  (params (OtherActor :type Actor%20Object%20Reference))
  ;[1 1 1] Use destroy event for auto explode after lifespan time
)

(event EventTick
  (params (DeltaSeconds :type Float%20%28single-precision%29)))

(event EventDestroyed
  ;[1 1 1] Use destroy event for auto explode after lifespan time
  (Debug|ShowDebugMessage "BaseProjectile_BP" "Destroyed" (Utilities|String|ToString(Name) (Utilities|Struct|BreakFProjectileWeaponData (Variables|UltimateCharacter|GetProjectileConfig))) "NewEnumerator0")
  ;[1 1 1] Event runs when projectile hit something
  (if (and (Utilities|Enum|Equal(Enum) (Networking|GetLocalRole) "ROLE_Authority") (not (Variables|Internal|GetbExploded)))
    (Debug|ShowDebugMessage "BaseProjectile_BP" "OnStopProjectile" (Utilities|String|Append (Utilities|String|ToString(Name) (Utilities|Struct|BreakFProjectileWeaponData (Variables|UltimateCharacter|GetProjectileConfig))) " stopped by " (Utilities|GetDisplayName (.HitActor (Collision|BreakHitResult (Variables|Internal|GetHitResult))))) "NewEnumerator0")
    (Explosion|Explode (Variables|Internal|GetHitResult))
    (Explosion|DisableandDestroy)))

(fn ConstructionScript)

(fn Initialize
  (bind _projectileconfig (Variables|UltimateCharacter|GetProjectileConfig))
  (bind _projectilemovement (Variables|Default|GetProjectileMovement))
  (bind _projectilecomponent (Utilities|Struct|BreakFProjectileWeaponData _projectileconfig))
  (bind (_initialspeed _maxspeed _projectilegravityscale _rotationfollowsvelocity _initialvelocityinlocalspace) (Utilities|Struct|BreakFProjectileComponent _projectilecomponent))
  (Debug|ShowDebugMessage "BaseProjectile_BP" "Initialize" (Utilities|String|Append (Utilities|String|ToString(Name) (Utilities|Struct|BreakFProjectileWeaponData (Variables|UltimateCharacter|GetProjectileConfig))) " initialized") "NewEnumerator0")
  ;[1 1 1] Set some default settings for projectile
  (Collision|IgnoreActorwhenMoving (Variables|Default|GetCollision) (Variables|Actor|GetInstigator) true)
  (Utilities|FlowControl|Sequence
    (:then_0
      (Variables|/Script/Engine.ProjectileMovementComponent|SetInitialSpeed _projectilemovement _initialspeed))
    (:then_1
      (Variables|/Script/Engine.ProjectileMovementComponent|SetMaxSpeed _projectilemovement _maxspeed))
    (:then_2
      (Variables|/Script/Engine.ProjectileMovementComponent|SetProjectileGravityScale _projectilemovement _projectilegravityscale))
    (:then_3
      (Variables|/Script/Engine.ProjectileMovementComponent|SetbRotationFollowsVelocity _projectilemovement _rotationfollowsvelocity))
    (:then_4
      (Variables|/Script/Engine.ProjectileMovementComponent|SetbInitialVelocityInLocalSpace _projectilemovement _initialvelocityinlocalspace)
      (if (Utilities|ClassIsChildOf (Utilities|GetClass (Components|GetOwner)) "/Game/UltimateCharacter/Blueprints/Weapons/Guns/ProjectileGun_BP.ProjectileGun_BP_C")
        _
        (else
          _))
      (Actor|SetLifeSpan (Utilities|Struct|BreakFProjectileWeaponData (Variables|UltimateCharacter|GetProjectileConfig)))
      (bind _asaicharacter_bp (Utilities|Casting|CastToAICharacter_BP (Game|GetInstigator)))
      (Variables|Internal|SetPawn_AI _asaicharacter_bp))))

(fn InitVelocity
  (bind _pawn_ai (Variables|Internal|GetPawn_AI))
  (bind _projectilemovement (Variables|Default|GetProjectileMovement))
  (bind _projectilemovement_2 (Variables|Default|GetProjectileMovement))
  (bind _controller_ai (Variables|/Game/UltimateCharacter/Blueprints/Characters/AICharacter_BP.AICharacter_BP_C|GetController_AI _pawn_ai))
  (bind _outtarget (Default|GetTarget _controller_ai))
  (bind _returnvalue (Transformation|GetVelocity _outtarget))
  (bind _returnvalue_2 (Math|Vector|VectorLength _returnvalue))
  (Debug|ShowDebugMessage "BaseProjectile_BP" "InitVelocity" (Utilities|String|ToString(Name) (Utilities|Struct|BreakFProjectileWeaponData (Variables|UltimateCharacter|GetProjectileConfig))) "NewEnumerator0")
  (if (Variables|UltimateCharacter|GetFlyToTarget)
    (Utilities|IsValid (Variables|Internal|GetPawn_AI)
      (:Is%20Valid
        ;[1 1 1] Read target data from BB
        (LocalVariables|SetTempStartLocation (Transformation|GetWorldLocation (Variables|Default|GetCollision)))
        (LocalVariables|SetTempEndLocation (Default|GetLastTargetLocation (Variables|/Game/UltimateCharacter/Blueprints/Characters/AICharacter_BP.AICharacter_BP_C|GetController_AI (Variables|Internal|GetPawn_AI))))
        (Utilities|IsValid (Default|GetTarget (Variables|/Game/UltimateCharacter/Blueprints/Characters/AICharacter_BP.AICharacter_BP_C|GetController_AI (Variables|Internal|GetPawn_AI)))
          (:Is%20Valid
            ;[1 1 1] Try to predict target location by his speed
            (if (> _returnvalue_2 0.0)
              (LocalVariables|SetTempEndLocation (+ (* (Transformation|GetActorForwardVector _outtarget) (/ _returnvalue_2 2.0)) (LocalVariables|GetTempEndLocation)))))
          (:Is%20Not%20Valid
            _))
        ;[1 1 1] Calculate projectile velocity to last target location
        (Variables|/Script/Engine.ProjectileMovementComponent|SetInitialSpeed (Variables|Default|GetProjectileMovement) (* (Math|Float|Clamp(Float) (Math|Vector|VectorLength (- (LocalVariables|GetTempStartLocation) (LocalVariables|GetTempEndLocation))) 1e+03 1e+04) (Variables|UltimateCharacter|GetSpeedMultiplier)))
        (bind _tossvelocity (Class|GameplayStatics|BlueprintSuggestProjectileVelocity (LocalVariables|GetTempStartLocation) (LocalVariables|GetTempEndLocation) (Variables|/Script/Engine.ProjectileMovementComponent|GetInitialSpeed (Variables|Default|GetProjectileMovement)) 0.0 "DoNotTrace" 0.0 false false))
        (bind _output_get (Variables|/Script/Engine.MovementComponent|SetVelocity _projectilemovement_2 _tossvelocity))
        (Components|Activation|Activate _projectilemovement_2 true)
        (Debug|ShowDebugMessage "BaseProjectile_BP" "InitVelocity" (Utilities|String|Append (Utilities|GetDisplayName self) " initialized velocity: " (Utilities|String|ToString(Vector) _output_get)) "NewEnumerator0"))
      (:Is%20Not%20Valid
        ;[1 1 1] Read projectile velocity from player character class
        (bind _asplayer_character_bp (Utilities|Casting|CastToPlayerCharacter_BP (Game|GetInstigator) :!label _label)
          (:then
            (bind _output_get_2 (Variables|/Script/Engine.MovementComponent|SetVelocity _projectilemovement (Variables|/Game/UltimateCharacter/Blueprints/Characters/PlayerCharacter_BP.PlayerCharacter_BP_C|GetThrowVelocity _asplayer_character_bp)))
            (Components|Activation|Activate _projectilemovement true)
            (Debug|ShowDebugMessage "BaseProjectile_BP" "InitVelocity" (Utilities|String|Append (Utilities|String|ToString(Name) (Utilities|Struct|BreakFProjectileWeaponData (Variables|UltimateCharacter|GetProjectileConfig))) " initialized velocity: " (Utilities|String|ToString(Vector) _output_get_2) " for player.") "NewEnumerator0"))
          (:CastFailed
            (Debug|ShowDebugMessage "BaseProjectile_BP" "InitVelocity" "Failed to cast to player or AI character" "NewEnumerator2")))))
    (else
      (goto _label))))

(fn Explode
  (params (InHit :type Hit%20Result%20Structure))
  (bind (_bblockinghit _binitialoverlap _time _distance _location _impactpoint _normal _impactnormal _physmat _hitactor) (Collision|BreakHitResult InHit))
  (bind _explosioneffect (Variables|UltimateCharacter|GetExplosionEffect))
  (bind _projectileconfig (Variables|UltimateCharacter|GetProjectileConfig))
  (bind _projectileconfig_2 (Variables|UltimateCharacter|GetProjectileConfig))
  (bind _projectileconfig_3 (Variables|UltimateCharacter|GetProjectileConfig))
  (bind _mesh (Variables|Default|GetMesh))
  (bind (_explosiondamage _damagetype) (Utilities|Struct|BreakFProjectileWeaponData _projectileconfig_3))
  (bind (_explosiondamage_2 _explosionradius _damagetype_2) (Utilities|Struct|BreakFProjectileWeaponData _projectileconfig))
  (bind (_explosiondamage_3 _explosionradius_2 _damagetype_3) (Utilities|Struct|BreakFProjectileWeaponData _projectileconfig_2))
  (bind _returnvalue (Transformation|GetWorldLocation _mesh))
  (bind _hitactor_2 (Collision|BreakHitResult InHit))
  (bind (_bblockinghit_2 _binitialoverlap_2 _time_2 _distance_2 _location_2 _impactpoint_2 _normal_2 _impactnormal_2) (Collision|BreakHitResult InHit))
  (Debug|ShowDebugMessage "BaseProjectile_BP" "Explode" (Utilities|String|Append (Utilities|String|ToString(Name) (Utilities|Struct|BreakFProjectileWeaponData (Variables|UltimateCharacter|GetProjectileConfig))) (Utilities|String|SelectString (Utilities|String|Append " hit " (Utilities|GetDisplayName _hitactor)) "" _bblockinghit)) "NewEnumerator0")
  (Utilities|FlowControl|Sequence
    (:then_0
      ;[1 1 1] Deactivate particle system
      (Utilities|IsValid (Variables|Default|GetParticle)
        (:Is%20Valid
          (Components|Activation|Deactivate (Variables|Default|GetParticle)))))
    (:then_1
      (LocalVariables|SetNudgedImpactLocation (Math|Vector|SelectVector _returnvalue (Math|Vector|SelectVector (+ _impactpoint_2 (* _impactnormal_2 1e+01)) _returnvalue _bblockinghit_2) (Physics|IsSimulatingPhysics _mesh "None"))))
    (:then_2
      ;[1 1 1] Apply radius damage & check block attack for characters
      (if (Math|Boolean|ANDBoolean (> _explosiondamage_2 0) (> _explosionradius 0.0) (Utilities|IsValidClass _damagetype_2))
        (if (Utilities|ClassIsChildOf (Utilities|GetClass _hitactor_2) "/Game/UltimateCharacter/Blueprints/Characters/BaseCharacter_BP.BaseCharacter_BP_C")
          (if (!= _hitactor_2 (Game|GetInstigator))
            ;;[1 1 1] Apply damage to the hitted actor directly using apply damage function to prevent problem with small radius
            (bind _asbase_character_bp (Utilities|Casting|CastToBaseCharacter_BP _hitactor_2)
              (:then
                (LocalVariables|SetTempCharacterHit _asbase_character_bp))
              (:CastFailed
                _))))
        (bind _outactors (Explosion|BlockCheck _explosionradius_2 (LocalVariables|GetTempCharacterHit)))
        (Game|Damage|ApplyRadialDamage (Math|Conversions|ToFloat(Integer) _explosiondamage_3) (LocalVariables|GetNudgedImpactLocation) _explosionradius_2 _damagetype_3 _outactors self (Game|GetInstigatorController) false "ECC_Visibility")
        ;[1 1 1] Apply damage to the hitted actor
        (Utilities|IsValid (LocalVariables|GetTempCharacterHit)
          (:Is%20Valid
            (bind (_boutblock _outdamagepercent) (Explosion|CanBlock (LocalVariables|GetTempCharacterHit)))
            (if _boutblock
              (bind _output_get (LocalVariables|SetTempDamagePercent _outdamagepercent))
              (if (> _output_get 0)
                (Game|Damage|ApplyDamage (LocalVariables|GetTempCharacterHit) (Math|Conversions|ToFloat(Integer) (/ (* _explosiondamage (LocalVariables|GetTempDamagePercent)) 100)) (Game|GetInstigatorController) self _damagetype :!label _label))
              (else
                (goto _label)))))))
    (:then_3
      ;[1 1 1] Spawn explosion effect
      (if (Utilities|IsValidClass _explosioneffect)
        (Debug|ShowDebugMessage "BaseProjectile_BP" "Explode" (Utilities|String|Append "Spawn explosion effect, " (Utilities|GetClassDisplayName _explosioneffect) " for " (Utilities|GetDisplayName self)) "NewEnumerator0")
        (bind _output_get_2 (LocalVariables|SetSpawnTransform (Math|Transform|MakeTransform (LocalVariables|GetNudgedImpactLocation) (Math|Conversions|RotationFromXVector (.ImpactPoint (Collision|BreakHitResult InHit))))))
        (bind _returnvalue_2 (Game|SpawnActorfromClass (Variables|UltimateCharacter|GetExplosionEffect) _output_get_2 "Undefined" "SelectDefaultAtRuntime" 0 0))
        (Utilities|IsValid _returnvalue_2
          (:Is%20Valid
            (Variables|/Game/UltimateCharacter/Blueprints/Effects/Explosions/ExplosionEffect_BP.ExplosionEffect_BP_C|SetSurfaceHit _returnvalue_2 InHit)))))
    (:then_4
      ;[1 1 1] Replicate explosion
      (Variables|Internal|SetbExploded true))
    (:then_5
      ;[1 1 1] If projectile life span is set to 0 change life spawn to small value then projectile will destory after a little time of expolsion
      (if (== (Utilities|Struct|BreakFProjectileWeaponData (Variables|UltimateCharacter|GetProjectileConfig)) 0.0)
        (Actor|SetLifeSpan 0.2)))))

(fn DisableandDestroy
  (bind _projectileconfig (Variables|UltimateCharacter|GetProjectileConfig))
  (bind _projectilelife (Utilities|Struct|BreakFProjectileWeaponData _projectileconfig))
  ;[1 1 1] Stop projectile from moving and set life span to destroy
  (Debug|ShowDebugMessage "BaseProjectile_BP" "DisableAndDestroy" (Utilities|String|ToString(Name) (Utilities|Struct|BreakFProjectileWeaponData (Variables|UltimateCharacter|GetProjectileConfig))) "NewEnumerator0")
  (Rendering|SetVisibility (Variables|Default|GetMesh) false false)
  (Components|Movement|StopMovementImmediately (Variables|Default|GetProjectileMovement))
  (Collision|SetCollisionEnabled (Variables|Default|GetCollision) "NoCollision")
  (if (== _projectilelife 0.0)
    (Actor|SetLifeSpan 0.2)
    (else
      (Actor|SetLifeSpan (Math|Float|Max(Float) _projectilelife 2.0)))))

(fn OnRepBExploded
  (bind _returnvalue (Transformation|GetActorForwardVector))
  (if (not (Utilities|Enum|Equal(Enum) (Networking|GetLocalRole) "ROLE_Authority"))
    (bind _returnvalue_2 (Collision|LineTraceByChannel (- (Transformation|GetActorLocation) (* _returnvalue 2e+02)) (+ (* _returnvalue 1.5e+02) (Transformation|GetActorLocation)) "TraceTypeQuery4" true (Utilities|Array|MakeArray (Variables|Actor|GetInstigator)) "None"))
    (if (not _returnvalue_2)
      (Explosion|Explode (Collision|MakeHitResult false false 0.0 0.0 "0, 0, 0" (Transformation|GetActorLocation) (* _returnvalue -1.0) "0,0,1" 0 0)))))

(fn ShowDebugMessage
  (params (InCallerName :type String) (InFunction :type String) (InMessage :type String) (InMessageType :type MessageType%20Enum :default "NewEnumerator0"))
  (if (or (Variables|UltimateCharacter-Debug|GetbShowDebug) (Utilities|Enum|Equal(Enum) InMessageType "NewEnumerator3"))
    (CallFunction|ShowDebugMessage InCallerName InFunction InMessage InMessageType)))

(fn BlockCheck
  (params (InRadius :type Float%20%28double-precision%29) (InHittedActor :type Base%20Character%20BP%20Object%20Reference))
  (Debug|ShowDebugMessage "BaseProjectile_BP" "BlockCheck" (Utilities|String|ToString(Name) (Utilities|Struct|BreakFProjectileWeaponData (Variables|UltimateCharacter|GetProjectileConfig))) "NewEnumerator0")
  ;[1 1 1] Don't run search for characters if radius is small
  (if (> InRadius 1e+02)
    (bind _outactors (Actor|GetAllActorsOfClass "/Game/UltimateCharacter/Blueprints/Characters/BaseCharacter_BP.BaseCharacter_BP_C"))
    (LocalVariables|SetTempAllCharacters _outactors)
    ;[1 1 1] Don't call block on instigator
    (bind _asbase_character_bp (Utilities|Casting|CastToBaseCharacter_BP (Game|GetInstigator))
      (:then
        (Utilities|Array|RemoveItem (LocalVariables|GetTempAllCharacters) _asbase_character_bp))
      (:CastFailed
        _))
    (Utilities|Array|RemoveItem (LocalVariables|GetTempAllCharacters) InHittedActor)
    (for _array_element (LocalVariables|GetTempAllCharacters)
      ;[1 1 1] We need to check characters inside the radius
      (LocalVariables|SetTempCharacter _array_element)
      (if (< (Math|Vector|VectorLength (- (Transformation|GetActorLocation) (Transformation|GetActorLocation _array_element))) InRadius)
        ;[1 1 1] Check line of sight from explosion to character
        (bind (_outhit _returnvalue) (Collision|LineTraceByChannel (Transformation|GetActorLocation) (Transformation|GetActorLocation (LocalVariables|GetTempCharacter)) "TraceTypeQuery1" false (Utilities|Array|MakeArray self) (select (Variables|UltimateCharacter-Debug|GetbShowDebug) "ForDuration" "None")))
        (if _returnvalue
          (if (== (.HitActor (Collision|BreakHitResult _outhit)) (LocalVariables|GetTempCharacter))
            (bind _boutblock (Explosion|CanBlock (LocalVariables|GetTempCharacter) :!label _label))
            (if _boutblock
              (Utilities|Array|AddUnique (LocalVariables|GetTempCharacters) (LocalVariables|GetTempCharacter)))
            (else
              (Debug|ShowDebugMessage "BaseProjectile_BP" "BlockCheck" (Utilities|String|Append (Utilities|GetDisplayName (.HitActor (Collision|BreakHitResult _outhit))) " blocks sight from " (Utilities|String|ToString(Name) (Utilities|Struct|BreakFProjectileWeaponData (Variables|UltimateCharacter|GetProjectileConfig))) " explosion to " (Utilities|String|ToString(Name) (Variables|/Game/UltimateCharacter/Blueprints/Characters/BaseCharacter_BP.BaseCharacter_BP_C|GetCharacterTag (LocalVariables|GetTempCharacter)))) "NewEnumerator3")))
          (else
            (goto _label))))))
  (Utilities|IsValid InHittedActor
    (:Is%20Valid
      ;[1 1 1] Make sure hitted actor is in ignore list
      (Utilities|Array|AddUnique (LocalVariables|GetTempCharacters) InHittedActor)
      (return (LocalVariables|GetTempCharacters)))
    (:Is%20Not%20Valid
      (return (LocalVariables|GetTempCharacters)))))

(fn CanBlock
  (params (InCharacter :type Base%20Character%20BP%20Object%20Reference))
  (bind _returnvalue (Components|GetOwner))
  (bind _returnvalue_2 (Components|GetOwner))
  (bind _returnvalue_3 (Utilities|GetClass _returnvalue))
  (Utilities|IsValid _returnvalue_2
    (:Is%20Valid
      (Debug|ShowDebugMessage "BaseProjectile_BP" "CanBlock" "" "NewEnumerator0")
      (bind _asaicharacter_bp (Utilities|Casting|CastToAICharacter_BP _returnvalue_2)
        (:then
          (if (.OutBlocked (Default|GetPlayerBlockedAttack _asaicharacter_bp))
            (return true (.OutDamagePercent (Default|GetPlayerBlockedAttack _asaicharacter_bp)))
            (else
              _)))
        (:CastFailed
          _))
      (Utilities|IsValid InCharacter
        (:Is%20Valid
          (if (Utilities|ClassIsChildOf _returnvalue_3 "/Game/UltimateCharacter/Blueprints/Characters/BaseCharacter_BP.BaseCharacter_BP_C")
            ;[1 1 1] If character will block the explosion add it to list
            (bind (_boutblocked _outdamagepercent) (Default|DoBlockAttack InCharacter "NewEnumerator5"))
            (return _boutblocked _outdamagepercent)
            (elif (Utilities|ClassIsChildOf _returnvalue_3 "/Game/UltimateCharacter/Blueprints/Weapons/BaseWeapon_BP.BaseWeapon_BP_C")
              (bind (_boutblocked_2 _outdamagepercent_2) (Default|DoBlockAttack InCharacter "NewEnumerator4"))
              (return _boutblocked_2 _outdamagepercent_2))))
        (:Is%20Not%20Valid
          (Debug|ShowDebugMessage "BaseProjectile_BP" "CanBlock" "Target character is not valid" "NewEnumerator0")
          (return false 100))))
    (:Is%20Not%20Valid
      (Debug|ShowDebugMessage "BaseProjectile_BP" "CanBlock" "Owner is not valid" "NewEnumerator0"))))